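; BP_Button is a VR button actor that responds to the ClickButton input action while a VRPawn is inside its box.
; Box overlaps open and close a gate, so a click calls ButtonClickMessage on the cached pawn only during overlap.
; The construction script sets arrow length and mesh height from ButtonOffset.
; Press animation is inactive: BeginPlay stores in/out transforms that go unused, and the MoveComponentTo logic is disconnected.
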(event OnComponentBeginOverlap(Box)
  (params (OverlappedComponent :type Primitive%20Component%20Object%20Reference) (OtherActor :type Actor%20Object%20Reference) (OtherComp :type Primitive%20Component%20Object%20Reference) (OtherBodyIndex :type Integer) (bFromSweep :type Boolean) (SweepResult :type Hit%20Result%20Structure%20%28by%20ref%29))
  (bind _asvrpawn (Utilities|Casting|CastToVRPawn OtherActor))
  (Utilities|FlowControl|Gate true) ; enters at Open
)

(event OnComponentEndOverlap(Box)
  (params (OverlappedComponent :type Primitive%20Component%20Object%20Reference) (OtherActor :type Actor%20Object%20Reference) (OtherComp :type Primitive%20Component%20Object%20Reference) (OtherBodyIndex :type Integer))
  (Utilities|Casting|CastToVRPawn OtherActor)
  (Utilities|FlowControl|Gate true) ; enters at Close
)

(event Input|EnhancedActionEvents|EnhancedInputActionClickButton
  (params (ActionValue :type Boolean) (ElapsedSeconds :type Float%20%28double-precision%29) (TriggeredSeconds :type Float%20%28double-precision%29) (InputAction :type Input%20Action%20Object%20Reference :default "/Game/Blueprints/Button/ClickButton.ClickButton"))
  (:Triggered
    (Utilities|FlowControl|Gate true
      (:Exit
        (Class|InteractInterface|ButtonClick(Message) (stale OnComponentBeginOverlap(Box) _asvrpawn))))))

(event EventBeginPlay
  (bind _staticmesh (Variables|Default|GetStaticMesh))
  (bind _returnvalue (Transformation|GetRelativeTransform _staticmesh))
  (Variables|Default|SetOut%20Position (Math|Transform|MakeTransform (.location _returnvalue) (.rotation _returnvalue) (.scale _returnvalue)))
  (Variables|Default|SetIn%20Position (Math|Transform|MakeTransform (- (.location _returnvalue) "0.000000,10.000000,0.000000") (.rotation _returnvalue) (.scale _returnvalue)))
  (Input|EnableInput (Game|GetPlayerController 0)))

(event EventTick
  (params (DeltaSeconds :type Float%20%28single-precision%29)))

(fn ConstructionScript
  (bind _buttonoffset (Variables|Default|GetButtonOffset))
  (Variables|/Script/Engine.ArrowComponent|SetArrowLength (Variables|Default|GetArrow) _buttonoffset)
  (Transformation|SetRelativeLocation (Variables|Default|GetStaticMesh) (Math|Vector|MakeVector 0.0 0.0 _buttonoffset) false false))