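; VR ladder actor that teleports the player's VRPawn on a click while in range of its bottom or top trigger box.
; Box overlaps set range flags, and the click passes the matching box (bottom checked first) to TeleportToLadder as the destination.
; That event plays a sound and a W_FadeToBlack animation, teleports, then reverses the fade.
; A TeleportedViaLadder flag blocks repeat teleports until a pawn leaves either box.
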(event OnComponentBeginOverlap(BoxBottom)
  (params (OverlappedComponent :type Primitive%20Component%20Object%20Reference) (OtherActor :type Actor%20Object%20Reference) (OtherComp :type Primitive%20Component%20Object%20Reference) (OtherBodyIndex :type Integer) (bFromSweep :type Boolean) (SweepResult :type Hit%20Result%20Structure%20%28by%20ref%29))
  ;[1 1 1] Teleport to other ladder end when entering Box Collision
  (Variables|Default|SetinBottomRange true))

(event OnComponentEndOverlap(BoxBottom)
  (params (OverlappedComponent :type Primitive%20Component%20Object%20Reference) (OtherActor :type Actor%20Object%20Reference) (OtherComp :type Primitive%20Component%20Object%20Reference) (OtherBodyIndex :type Integer))
  ;[1 1 1] Set bool so that player does not end in a teleport loop
  (Utilities|Casting|CastToPawn (stale OnComponentEndOverlap(BoxTop) OtherActor))
  (Variables|Default|SetteleportedViaLadder false)
  (Variables|Default|SetinBottomRange false))

(event OnComponentBeginOverlap(BoxTop)
  (params (OverlappedComponent :type Primitive%20Component%20Object%20Reference) (OtherActor :type Actor%20Object%20Reference) (OtherComp :type Primitive%20Component%20Object%20Reference) (OtherBodyIndex :type Integer) (bFromSweep :type Boolean) (SweepResult :type Hit%20Result%20Structure%20%28by%20ref%29))
  ;[1 1 1] Teleport to other ladder end when entering Box Collision
  (Variables|Default|SetinTopRange true))

(event OnComponentEndOverlap(BoxTop)
  (params (OverlappedComponent :type Primitive%20Component%20Object%20Reference) (OtherActor :type Actor%20Object%20Reference) (OtherComp :type Primitive%20Component%20Object%20Reference) (OtherBodyIndex :type Integer))
  ;[1 1 1] Set bool so that player does not end in a teleport loop
  (Utilities|Casting|CastToPawn OtherActor)
  (Variables|Default|SetteleportedViaLadder false)
  (Variables|Default|SetinTopRange false))

(event Custom|TeleportToLadder
  (params (VRPawn :type Object%20Object%20Reference) (BoxPlayerTeleportsTo :type Scene%20Component%20Object%20Reference))
  ;[1 1 1] Teleport when entering Box Collision and play fade in/out animations
  (if (not (Variables|Default|GetteleportedViaLadder))
    (bind _asvrpawn (Utilities|Casting|CastToVRPawn VRPawn))
    (Variables|Default|SetteleportedViaLadder true)
    ;;[1 1 1] play sound and fade to black animation
    (Audio|PlaySoundatLocation "/Game/Sounds/Soundeffects/Ladder_Cue.Ladder_Cue" "0, 0, 0" "0, 0, 0" 1.0 1.0 0.0 0 0 0 0)
    (bind _returnvalue (UserInterface|CreateWidget "/Game/UI/W_FadeToBlack.W_FadeToBlack_C" (Game|GetPlayerController 0)))
    (Components|Animation|PlayAnimation _returnvalue (Variables|/Game/UI/W_FadeToBlack.W_FadeToBlack_C|GetFadeInBlack _returnvalue) 0.0
      (:Finished
        ;;[1 1 1] Teleport player
        (Transformation|Teleport _asvrpawn (Transformation|GetWorldLocation BoxPlayerTeleportsTo) (Transformation|GetWorldRotation BoxPlayerTeleportsTo))
        ;;[1 1 1] Play fade out from black animation
        (Components|Animation|PlayAnimation _returnvalue (Variables|/Game/UI/W_FadeToBlack.W_FadeToBlack_C|GetFadeInBlack _returnvalue) 0.0 1 "Reverse")))))

(event Input|EnhancedActionEvents|EnhancedInputActionClickButton
  (params (ActionValue :type Boolean) (ElapsedSeconds :type Float%20%28double-precision%29) (TriggeredSeconds :type Float%20%28double-precision%29) (InputAction :type Input%20Action%20Object%20Reference :default "/Game/Blueprints/Button/ClickButton.ClickButton"))
  ;[1 1 1] Teleport when pressing the click button
  (:Started
    (if (Variables|Default|GetinBottomRange)
      (CallFunction|TeleporttoLadder (stale OnComponentBeginOverlap(BoxBottom) OtherActor) (Variables|Default|GetBoxBottom))
      (elif (Variables|Default|GetinTopRange)
        (CallFunction|TeleporttoLadder (stale OnComponentBeginOverlap(BoxTop) OtherActor) (Variables|Default|GetBoxTop))))))

(event EventBeginPlay)

(event Collision|EventActorBeginOverlap
  (params (OtherActor :type Actor%20Object%20Reference)))

(event EventTick
  (params (DeltaSeconds :type Float%20%28single-precision%29)))

(fn ConstructionScript)