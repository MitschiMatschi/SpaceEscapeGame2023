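; BP_Quizz is an in-world quiz display that shows German space-history questions, each with three numbered answers, on a TextRender component.
; The NextQuestion event, intended to fire after a correct answer, increments CurrentQuestion and switches on it to set the next hardcoded question or a final all-correct message.
; Answer checking is not in this Blueprint, and BeginPlay, overlap and Tick are unused.
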(event Custom|NextQuestion
  ;[1 1 1] Text changes to next question when player selected the right answer
  (bind _output_get (Variables|Default|SetCurrentQuestion (+ (Variables|Default|GetCurrentQuestion) 1)))
  (switch int _output_get
    (:Default
      (Rendering|Components|TextRender|SetText (Variables|Default|GetTextRender) (Utilities|Text|MakeLiteralText "In welchem Jahr fand die Mondlandung statt? 
1) 1951 
2) 1996 
3) 1969") :!label _label))
    (:1
      (goto _label))
    (:2
      (Rendering|Components|TextRender|SetText (Variables|Default|GetTextRender) (Utilities|Text|MakeLiteralText "Wer war der erste Mensch im Weltall? 
1) Juri Gagarin 
2) Elon Musk 
3) Neil Armstrong")))
    (:3
      (Rendering|Components|TextRender|SetText (Variables|Default|GetTextRender) (Utilities|Text|MakeLiteralText "Welches Lebewesen wurde als erstes  
gezielt in die Erdumlaufbahn gebracht? 
1) Schimpanse 
2) Hündin 
3) Hamster")))
    (:4
      (Rendering|Components|TextRender|SetText (Variables|Default|GetTextRender) (Utilities|Text|MakeLiteralText "Alle Fragen korrekt beantwortet!")))))

(event EventBeginPlay)

(event Collision|EventActorBeginOverlap
  (params (OtherActor :type Actor%20Object%20Reference)))

(event EventTick
  (params (DeltaSeconds :type Float%20%28single-precision%29)))

(fn ConstructionScript)