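; BP_SlotQuizz is a puzzle slot that checks slotted actors as answers to a three-question quiz.
; IsCorrectActor compares the minigame ID and the current question's expected actor ID, playing a confirmation or wrong-answer sound.
; Correct answers call NextQuestion on the quiz reference, and the third also notifies the puzzle manager using the slot's first tag.
; The check always returns false, leaving the actor removable from the slot.
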(event EventBeginPlay
  (|CallParentFunction) ; This node is disabled and will not be called.\nDrag off pins to build functionality.
)

(event Collision|EventActorBeginOverlap
  (params (OtherActor :type Actor%20Object%20Reference)))

(event EventTick
  (params (DeltaSeconds :type Float%20%28single-precision%29)))

(fn ConstructionScript
  (|CallParentFunction))

(fn IsCorrectActor
  (params (InputActorID :type Integer) (InputMinigameID :type String))
  (switch int (Variables|Default|GetCurrentQuizzQuestion)
    (:Default
      (if (and (Utilities|Enum|Equal(Enum) InputMinigameID (Variables|Default|GetCorrectMinigame%20ID)) (== InputActorID (Variables|Default|GetCorrectActorID))) :!label _label
        ;[1 1 1] Correct Answer
        (Variables|Default|SetSlotCorrectlyInUse true :!label _label_2)
        (Development|PrintString "Correct ID, yay :D")
        (Variables|Default|SetCurrentQuizzQuestion (+ (Variables|Default|GetCurrentQuizzQuestion) 1))
        (Audio|PlaySoundatLocation "/Game/Sounds/Soundeffects/Confirmation_Cue.Confirmation_Cue" (Transformation|GetActorLocation) "0, 0, 0" 1.0 1.0 0.0 0 0 0 0)
        (Default|NextQuestion (Variables|Default|GetQuizzReference))
        (else
          ;[1 1 1] Wrong
          (Development|PrintString "Wrong ID..." :!label _label_3)
          (Audio|PlaySoundatLocation "/Game/Sounds/Soundeffects/Wrong_Answer_Cue.Wrong_Answer_Cue" (Transformation|GetActorLocation) "0, 0, 0" 1.0 1.0 0.0 0 0 0 0))))
    (:1
      (goto _label))
    (:2
      (if (and (Utilities|Enum|Equal(Enum) InputMinigameID (Variables|Default|GetCorrectMinigame%20ID)) (== InputActorID (Variables|Default|GetCorrect%20ID%202)))
        (goto _label_2)
        (else
          (goto _label_3))))
    (:3
      (if (and (Utilities|Enum|Equal(Enum) InputMinigameID (Variables|Default|GetCorrectMinigame%20ID)) (== InputActorID (Variables|Default|GetCorrect%20ID%203)))
        ;[1 1 1] ALL Questions answered correctly, send to puzzle manager that quizz is completed
        (Variables|Default|SetSlotCorrectlyInUse true)
        (Development|PrintString "ALL QUIZZ QUESTIONS CORRECT")
        (Default|NextQuestion (Variables|Default|GetQuizzReference))
        (Default|OnCorrectlySlotted (Variables|Default|GetPuzzleManagerRef) (Utilities|Array|Get(acopy) (Variables|Default|GetTags)))
        (Audio|PlaySoundatLocation "/Game/Sounds/Soundeffects/Confirmation_Cue.Confirmation_Cue" (Transformation|GetActorLocation) "0, 0, 0" 1.0 1.0 0.0 0 0 0 0)
        (else
          (goto _label_3)))))
  ;[1 1 1] Is Actor Correct --> when false, able to take out slottable actor from slot
  (return false))