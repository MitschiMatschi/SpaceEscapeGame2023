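; BP_Light is a toggleable light actor built from three spot light components.
; Its Lighton event flips the IsOn flag, applies it to the visibility of all three spot lights and prints a debug "Light on" message regardless of the new state.
; The construction script applies the same flag, so the lights match the initial IsOn value.
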(event EventLighton
  (bind _output_get (Variables|Default|SetIsOn? (not (Variables|Default|GetIsOn?))))
  (Rendering|SetVisibility (Variables|Default|GetSpotLight1) _output_get false)
  (Development|PrintString "Light on" true true "(R=1.000000,G=0.125040,B=0.848857,A=1.000000)"))

(fn ConstructionScript
  (Rendering|SetVisibility (Variables|Default|GetSpotLight1) (Variables|Default|GetIsOn?) false))