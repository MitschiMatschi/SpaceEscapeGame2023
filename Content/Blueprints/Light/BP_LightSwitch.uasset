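; BP_LightSwitch is a VR light switch actor that turns on the BP_Light actors sharing its LightIndex.
; At BeginPlay it caches every BP_Light in the level.
; A VRPawn entering or leaving its Box toggles input and a gate on the ClickButton action.
; A click plays a switch sound and sends LightOnMessage to each matching light; there is no off path, and debug prints remain throughout.
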(event OnComponentBeginOverlap(Box)
  (params (OverlappedComponent :type Primitive%20Component%20Object%20Reference) (OtherActor :type Actor%20Object%20Reference) (OtherComp :type Primitive%20Component%20Object%20Reference) (OtherBodyIndex :type Integer) (bFromSweep :type Boolean) (SweepResult :type Hit%20Result%20Structure%20%28by%20ref%29))
  ;[1 1 1] Switch on all the lights
  (Utilities|Casting|CastToVRPawn OtherActor)
  (Development|PrintString "AAAAAAAAAAAAAAAAAAAAAAAAAAAAAAAAAA" true true "(R=0.066667,G=1.000000,B=0.398625,A=1.000000)")
  (Input|EnableInput self (Game|GetPlayerController 0))
  (Utilities|FlowControl|Gate true) ; enters at Open
)

(event OnComponentEndOverlap(Box)
  (params (OverlappedComponent :type Primitive%20Component%20Object%20Reference) (OtherActor :type Actor%20Object%20Reference) (OtherComp :type Primitive%20Component%20Object%20Reference) (OtherBodyIndex :type Integer))
  ;[1 1 1] Switch on all the lights
  (Utilities|Casting|CastToVRPawn OtherActor)
  (Input|DisableInput self (Game|GetPlayerController 0))
  (Utilities|FlowControl|Gate true) ; enters at Close
)

(event Input|EnhancedActionEvents|EnhancedInputActionClickButton
  (params (ActionValue :type Boolean) (ElapsedSeconds :type Float%20%28double-precision%29) (TriggeredSeconds :type Float%20%28double-precision%29) (InputAction :type Input%20Action%20Object%20Reference :default "/Game/Blueprints/Button/ClickButton.ClickButton"))
  ;[1 1 1] Switch on all the lights
  (:Started
    (Development|PrintString "ClickButton" true true "(R=1.000000,G=0.373446,B=0.518090,A=1.000000)")
    (Utilities|FlowControl|Gate true
      (:Exit
        (for _array_element (Variables|Default|GetLightsArray)
          (if (== (Variables|/Game/Blueprints/Light/BP_Light.BP_Light_C|GetLightIndex _array_element) (Variables|Default|GetLight%20Index%20))
            (Audio|PlaySoundatLocation "/Game/Sounds/Soundeffects/Light_switch_Cue.Light_switch_Cue" (Transformation|GetWorldLocation (Variables|Default|GetCube)) "0, 0, 0" 1.0 1.0 0.0 0 0 0 0)
            (Class|LightInterface|Lighton(Message) _array_element)
            (Development|PrintString "Light on")))
        (Development|PrintString "Loop ended" true true "(R=1.000000,G=0.944914,B=0.463292,A=1.000000)")))))

(event EventBeginPlay
  ;[1 1 1] Get all the lights in the level
  (bind _outactors (Actor|GetAllActorsOfClass "/Game/Blueprints/Light/BP_Light.BP_Light_C"))
  (for _array_element _outactors
    (bind _returnvalue (Utilities|Array|Add (Variables|Default|GetLightsArray) _array_element))
    (Development|PrintString (Utilities|String|ToString(Integer) _returnvalue))))

(fn ConstructionScript)