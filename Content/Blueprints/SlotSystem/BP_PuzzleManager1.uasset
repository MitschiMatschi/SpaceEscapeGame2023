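; Puzzle manager actor that detects when tagged slot puzzles are complete and triggers their completion responses.
; OnCorrectlySlotted checks that every BP_Slot with the given tag is correctly filled.
; On completion it briefly sets IsSuccess on the cached Robot_BP, then switches on the tag to per-puzzle events that only print messages, with unknown tags falling back to Test.
; A separate GameWon event plays a countdown sound at the manager's location.
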(event Custom|TestCompletion
  ;[1 1 1] On puzzle completion
  (Development|PrintString "Test Puzzle COMPLETED" true true "(R=1.000000,G=0.000000,B=0.971477,A=1.000000)"))

(event Custom|OnCorrectlySlotted
  (params (Tag :type Name))
  ;[1 1 1] On correctly slotted --> if puzzle complete call the <tag> completion function
  (bind _complete (CallFunction|CheckifPuzzleComplete Tag))
  (if _complete
    (CallFunction|DefaultCompletion)
    (switch name Tag
      (:Default
        (CallFunction|TestCompletion :!label _label))
      (:Test
        (goto _label))
      (:Quizz
        (CallFunction|QuizzCompletion))
      (:PlantSeeds
        (CallFunction|PlantSeedsCompletion))
      (:Repair
        (CallFunction|RepairCompletion))
      (:Analyzer
        (CallFunction|AnalyzerCompletion)))))

(event Custom|DefaultCompletion
  (bind _robotref (Variables|Default|GetRobotRef))
  ;[1 1 1] Happens for every puzzle
  (Variables|/Game/Robot/Blueprints/Robot_BP.Robot_BP_C|SetisSuccess _robotref true)
  (Utilities|FlowControl|Delay 1.68)
  (Variables|/Game/Robot/Blueprints/Robot_BP.Robot_BP_C|SetisSuccess _robotref false))

(event Custom|QuizzCompletion
  ;[1 1 1] On Quizz completion
  (Development|PrintString "Quizz COMPLETED" true true "(R=1.000000,G=0.000000,B=0.971477,A=1.000000)"))

(event Custom|PlantSeedsCompletion
  ;[1 1 1] On Plant Seeds completion
  (Development|PrintString "Plant Seeds COMPLETED" true true "(R=1.000000,G=0.000000,B=0.971477,A=1.000000)"))

(event Custom|RepairCompletion
  ;[1 1 1] On Repair Completed
  (Development|PrintString "Repair COMPLETED" true true "(R=1.000000,G=0.000000,B=0.971477,A=1.000000)"))

(event Custom|AnalyzerCompletion
  ;[1 1 1] On Analyzer Completed
  (Development|PrintString "Analyzer COMPLETED" true true "(R=1.000000,G=0.000000,B=0.971477,A=1.000000)"))

(event Custom|GameWon
  ;[1 1 1] When you win the game, play countdown
  (Audio|PlaySoundatLocation "/Game/Sounds/Soundeffects/Countdown_Cue.Countdown_Cue" (Transformation|GetActorLocation) "0, 0, 0" 1.0 1.0 0.0 0 0 0 0))

(event EventBeginPlay
  ;[1 1 1] Get robot ref
  (bind _returnvalue (Actor|GetActorOfClass "/Game/Robot/Blueprints/Robot_BP.Robot_BP_C"))
  (Variables|Default|SetRobotRef _returnvalue))

(fn ConstructionScript)

(fn CheckifPuzzleComplete
  (params (Tag :type Name))
  ;[1 1 1] Returns true if all puzzles of TAG are completed (all slots are filled correctly)
  (bind _outactors (Actor|GetAllActorsOfClasswithTag "/Game/Blueprints/SlotSystem/BP_Slot.BP_Slot_C" Tag))
  (for _array_element _outactors
    (if (not (Variables|/Game/Blueprints/SlotSystem/BP_Slot.BP_Slot_C|GetSlotCorrectlyInUse _array_element))
      (return false)))
  (return true))