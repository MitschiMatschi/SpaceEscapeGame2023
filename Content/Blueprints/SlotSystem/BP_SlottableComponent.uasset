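; Actor component that lets a grabbable puzzle actor snap into and out of BP_Slot actors.
; On drop, or via a debug delay after BeginPlay, it snaps its owner to the nearest in-range slot if free, keeping mesh scale and disabling physics.
; The slot checks actor and minigame IDs for correctness.
; Grabbing detaches and restores physics only when IsActorCorrect is true, although the inline comment states the opposite.
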(event Custom|SnapToSlot
  (bind _returnvalue (Components|GetOwner))
  (bind _slotsinrange (Variables|Default|GetSlotsInRange))
  (bind _returnvalue_2 (Actor|GetComponentbyClass _returnvalue "/Script/Engine.StaticMeshComponent"))
  ;[1 1 1] If actor (with grab component) is dropped in range of slot, snap to closest one
  (if (Utilities|Array|IsNotEmpty _slotsinrange)
    (bind _asbp_slot (Utilities|Casting|CastToBP_Slot (.ReturnValue (Actor|FindNearestActor (Transformation|GetWorldLocation (Variables|Default|GetGrabComponentRef)) _slotsinrange))))
    (bind _output_get (Variables|Default|SetAttachedSlot _asbp_slot))
    ;;[1 1 1] only snap if slot is free
    (Utilities|IsValid _output_get
      (:Is%20Valid
        (if (not (Variables|/Game/Blueprints/SlotSystem/BP_Slot.BP_Slot_C|GetSlotInUse _output_get))
          ;;[1 1 1] get the transform of closest slot
          (Transformation|SetActorTransform (Components|GetOwner) (Math|Transform|MakeTransform (.location (Transformation|GetActorTransform _output_get)) (.rotation (Transformation|GetActorTransform _output_get)) (.scale (Transformation|GetWorldTransform _returnvalue_2))))
          (Default|AttachtoSlot (Variables|Default|GetAttachedSlot))
          ;;[1 1 1] Actor will not move from slot
          (Physics|SetSimulatePhysics _returnvalue_2 false)
          (Development|PrintString "SNAP!")
          ;;[1 1 1] Check if it is the correct actor to solve the puzzle
          (bind _isactorcorrect (Default|IsCorrectActor (Variables|Default|GetAttachedSlot) (Variables|Default|GetID) (Variables|Default|GetMinigameID)))
          (Variables|Default|SetIsActorCorrect _isactorcorrect))))))

(event Custom|DetachFromSlot
  (bind _attachedslot (Variables|Default|GetAttachedSlot))
  ;[1 1 1] if actor (with grab and slottable components) is grabbed from slot, detach from slot
  ;;[1 1 1] ONLY if you haven't slotted the correct actor
  (if (Variables|Default|GetIsActorCorrect)
    ;;[1 1 1] Detach from slot
    (Utilities|IsValid _attachedslot
      (:Is%20Valid
        (Default|DetachfromSlot _attachedslot)
        ;;[1 1 1] Reactivate physics
        (Physics|SetSimulatePhysics (Actor|GetComponentbyClass (Components|GetOwner) "/Script/Engine.StaticMeshComponent") true)))))

(event EventBeginPlay
  (bind _returnvalue (Components|GetOwner))
  (bind _returnvalue_2 (Components|GetOwner))
  (bind _slotsinrange (Variables|Default|GetSlotsInRange))
  (bind _returnvalue_3 (Actor|GetComponentbyClass _returnvalue "/Script/Engine.StaticMeshComponent"))
  ;[1 1 1] get the grab component of parent
  (bind _output_get (Variables|Default|SetGrabComponentRef (Actor|GetComponentbyClass _returnvalue_2 "/Game/VRTemplate/Blueprints/GrabComponent.GrabComponent_C")))
  (EventDispatchers|BindEventtoOnDropped _output_get (delegate Custom|SnapToSlot))
  (EventDispatchers|BindEventtoOnGrabbed _output_get (delegate Custom|DetachFromSlot))
  ;[1 0.309 0] DEBUG ONLY
  (Utilities|FlowControl|Delay 1e+01)
  ;[1 1 1] If actor (with grab component) is dropped in range of slot, snap to closest one
  (if (Utilities|Array|IsNotEmpty _slotsinrange)
    (bind _asbp_slot (Utilities|Casting|CastToBP_Slot (.ReturnValue (Actor|FindNearestActor (Transformation|GetWorldLocation (Variables|Default|GetGrabComponentRef)) _slotsinrange))))
    (bind _output_get_2 (Variables|Default|SetAttachedSlot _asbp_slot))
    ;;[1 1 1] only snap if slot is free
    (Utilities|IsValid _output_get_2
      (:Is%20Valid
        (if (not (Variables|/Game/Blueprints/SlotSystem/BP_Slot.BP_Slot_C|GetSlotInUse _output_get_2))
          ;;[1 1 1] get the transform of closest slot
          (Transformation|SetActorTransform _returnvalue_2 (Math|Transform|MakeTransform (.location (Transformation|GetActorTransform _output_get_2)) (.rotation (Transformation|GetActorTransform _output_get_2)) (.scale (Transformation|GetWorldTransform _returnvalue_3))))
          (Default|AttachtoSlot (Variables|Default|GetAttachedSlot))
          ;;[1 1 1] Actor will not move from slot
          (Physics|SetSimulatePhysics _returnvalue_3 false)
          (Development|PrintString "SNAP!")
          ;;[1 1 1] Check if it is the correct actor to solve the puzzle
          (bind _isactorcorrect (Default|IsCorrectActor (Variables|Default|GetAttachedSlot) (Variables|Default|GetID) (Variables|Default|GetMinigameID)))
          (Variables|Default|SetIsActorCorrect _isactorcorrect))))))