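; BP_Slot is a placement slot, apparently for puzzles, that previews slottable actors entering its resizable collision box as a ghost mesh.
; Overlapping actors with BP_SlottableComponent are tracked in an array and the slot registers itself on their component; the ghost shows the newest one.
; Attach and detach events only toggle the in-use flag and ghost visibility, while IsCorrectActor compares an ID against the expected one.
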(event OnComponentBeginOverlap(BoxCollision)
  (params (OverlappedComponent :type Primitive%20Component%20Object%20Reference) (OtherActor :type Actor%20Object%20Reference) (OtherComp :type Primitive%20Component%20Object%20Reference) (OtherBodyIndex :type Integer) (bFromSweep :type Boolean) (SweepResult :type Hit%20Result%20Structure%20%28by%20ref%29))
  (bind _returnvalue (Actor|GetComponentbyClass OtherActor "/Game/Blueprints/SlotSystem/BP_SlottableComponent.BP_SlottableComponent_C"))
  ;[1 1 1 1 25] On overlap with a slottable actor --> show the ghost mesh, in slot range true
  ;;[1 1 1] Only do if slot is free (NOT in use)
  (if (not (Variables|Default|GetSlotInUse))
    (Utilities|IsValid _returnvalue
      (:Is%20Valid
        (Variables|Default|SetSlottableComponentRef _returnvalue)
        (bind _output_get (Variables|Default|SetNewestSlottableActor OtherActor))
        (Utilities|Array|Add (Variables|Default|GetSlottablesInRange) _output_get)
        (CallFunction|UpdateGhostMesh _output_get)
        (Utilities|IsValid (Variables|Default|GetSlottableComponentRef)
          (:Is%20Valid
            (Utilities|Array|Add (Variables|/Game/Blueprints/SlotSystem/BP_SlottableComponent.BP_SlottableComponent_C|GetSlotsInRange (Variables|Default|GetSlottableComponentRef)) self)
            ;;[1 0.4965 0] DEBUG
            (if true
              (Development|PrintString "overlap: in slot range true")
              (else
                (Development|PrintString "overlap: in slot range false")))))))))

(event OnComponentEndOverlap(BoxCollision)
  (params (OverlappedComponent :type Primitive%20Component%20Object%20Reference) (OtherActor :type Actor%20Object%20Reference) (OtherComp :type Primitive%20Component%20Object%20Reference) (OtherBodyIndex :type Integer))
  (bind _slottablesinrange (Variables|Default|GetSlottablesInRange))
  ;[1 1 1 1 25] On end overlap with a slottable object (if it is the same as the On Overlap one) --> stop showing ghost mesh, in slot range false
  ;;[1 1 1] Only do if slot is free (unoccupied)
  (if (not (Variables|Default|GetSlotInUse))
    (if (Utilities|Array|ContainsItem (Variables|Default|GetSlottablesInRange) OtherActor)
      ;;[1 1 1] if actor with slot component ends overlap with BP_Slot, BP_Slot will remove its reference to the component
      (bind _output_get (Variables|Default|SetSlottableComponentRef (Actor|GetComponentbyClass OtherActor "/Game/Blueprints/SlotSystem/BP_SlottableComponent.BP_SlottableComponent_C")))
      (Utilities|Array|RemoveItem (Variables|/Game/Blueprints/SlotSystem/BP_SlottableComponent.BP_SlottableComponent_C|GetSlotsInRange _output_get) self)
      (if (== OtherActor (Variables|Default|GetNewestSlottableActor))
        ;;[1 1 1] if newest slottable actor left range, remove from array and show the "new" newest slottable actor
        ;;;[1 1 1] set the last actor (in slottablesInRange array) as the newest slottable actor
        (bind _returnvalue (Utilities|Array|RemoveItem (Variables|Default|GetSlottablesInRange) (Variables|Default|GetNewestSlottableActor)))
        (Development|PrintString "Newest slottable actor removed from slottables in range" _returnvalue)
        (Variables|Default|SetNewestSlottableActor (Utilities|Array|Get(acopy) _slottablesinrange (Utilities|Array|LastIndex _slottablesinrange)))
        ;;;[1 1 1] if no slottables in range, ghost mesh is invisible (has no mesh)
        (if (Utilities|Array|IsEmpty (Variables|Default|GetSlottablesInRange))
          (Components|StaticMesh|SetStaticMesh (Variables|Components|GetGhostMesh) 0)
          (else
            (CallFunction|UpdateGhostMesh (Variables|Default|GetNewestSlottableActor))))
        (else
          ;;[1 1 1] if actor who left range is not the newest one, remove from array
          ;;;[1 1 1] delete this actor from slottables in range
          (bind _returnvalue_2 (Utilities|Array|RemoveItem (Variables|Default|GetSlottablesInRange) OtherActor))
          (Development|PrintString "Slottable actor removed from slottables in range" _returnvalue_2)
          (CallFunction|UpdateGhostMesh (Variables|Default|GetNewestSlottableActor)))))))

(event Custom|UpdateGhostMesh
  (params (SlottableActor :type Actor%20Object%20Reference))
  (bind _returnvalue (Actor|GetComponentbyClass SlottableActor "/Script/Engine.StaticMeshComponent"))
  (bind _ghostmesh (Variables|Components|GetGhostMesh))
  ;[1 1 1 1 25] UpdateGhostMesh
  ;;[1 1 1] set the ghost mesh to look like the slottable actor's mesh
  (Components|StaticMesh|SetStaticMesh _ghostmesh (Variables|/Script/Engine.StaticMeshComponent|GetStaticMesh _returnvalue))
  (Transformation|SetWorldScale3D _ghostmesh (Transformation|GetWorldScale _returnvalue))
  (Rendering|SetVisibility _ghostmesh true false)
  ;;[1 1 1] Set ghost material
  (for _index (range 0 (- (Rendering|Material|GetNumMaterials _ghostmesh) 1))
    (Rendering|Material|SetMaterial _ghostmesh _index (Variables|Default|GetGhostMaterial))))

(event Custom|DetachFromSlot
  ;[1 1 1 1 25] Attach and detach from slot --> only set visibility and slotInUse
  (Variables|Default|SetSlotInUse false)
  (Rendering|SetVisibility (Variables|Components|GetGhostMesh) true false)
  (Development|PrintString "detach to slot"))

(event Custom|AttachToSlot
  ;[1 1 1 1 25] Attach and detach from slot --> only set visibility and slotInUse
  (Variables|Default|SetSlotInUse true)
  (Rendering|SetVisibility (Variables|Components|GetGhostMesh) false false)
  (Development|PrintString "attach to slot"))

(fn ConstructionScript
  ;[1 1 1] Change size of box collision in level
  (Components|Box|SetBoxExtent (Variables|Components|GetBoxCollision) (Variables|Default|GetBoxCollisionSize) true))

(fn IsCorrectActor
  (params (InputActorID :type Integer))
  (bind _correctactorid (Variables|Default|GetCorrectActorID))
  (bind _returnvalue (== InputActorID _correctactorid))
  ;[0.9821 0.4948 1] Implement functionality for CorrectActor (is it the correct one? if yes, you solved the puzzle
  (if _returnvalue
    (Development|PrintString "Correct ID, yay :D")
    (else
      (Development|PrintString "Wrong ID...")))
  (return _returnvalue))