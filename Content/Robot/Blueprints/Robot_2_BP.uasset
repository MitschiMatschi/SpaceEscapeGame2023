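; Robot actor that chases the Ball_BP actor through AI movement.
; On BeginPlay it finds the ball, starts the follow loop and plays its audio.
; FollowBall re-runs itself after a short delay while its flag is set, moving toward the ball or targeting itself to hold position when already close.
; An older look-at rotation system remains unconnected.
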(event Custom|Follow%20Ball
  (bind _ball (Variables|Default|GetBall))
  ;[1 1 1] Move towards player
  (if (Variables|Default|GetFollow%20Ball?)
    (if (>= (Transformation|GetDistanceTo _ball) 2e+01)
      (AI|AIMoveTo self "0, 0, 0" _ball 1e+01 false
        (:then
          _))
      (else
        (AI|AIMoveTo self "0, 0, 0" self 1e+01 false
          (:then
            _))))
    ;[1 1 1] Look at player
    (Utilities|FlowControl|Delay 0.1)
    (CallFunction|FollowBall)))

(event EventBeginPlay
  ;[1 1 1] Get ball ref
  (bind _returnvalue (Actor|GetActorOfClass "/Game/Props/Blueprints/Ball_BP.Ball_BP_C"))
  (Variables|Default|SetBall _returnvalue)
  (CallFunction|FollowBall)
  (Audio|Components|Audio|Play (Variables|Default|GetAudio) 0.0)
  (Audio|Components|Audio|Play (Variables|Default|GetAudio) 0.0))

(fn ConstructionScript)