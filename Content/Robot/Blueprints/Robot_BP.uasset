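; Robot character that follows the VR player around using AI navigation.
; On BeginPlay it caches the VRPawn, then re-runs FollowPlayer on a short delay for as long as its follow flag is set.
; Beyond a distance threshold it moves toward the player; when closer, it targets itself to hold position.
; Tick's velocity check does nothing, and the turn-to-face-player logic is disconnected.
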(event Custom|Follow%20Player
  (bind _vrpawn (Variables|Default|GetVRPawn))
  ;[1 1 1] Move towards player
  (if (Variables|Default|GetFollow%20Player?)
    (if (>= (Transformation|GetDistanceTo _vrpawn) 4e+02)
      (AI|AIMoveTo self "0, 0, 0" _vrpawn 1e+01 false
        (:then
          _))
      (else
        (AI|AIMoveTo self "0, 0, 0" self 1e+01 false
          (:then
            _))))
    ;[1 1 1] Look at player
    (Utilities|FlowControl|Delay 0.2)
    (CallFunction|FollowPlayer)))

(event EventBeginPlay
  ;[1 1 1] Get player reference
  (bind _asvrpawn (Utilities|Casting|CastToVRPawn (Game|Player|GetPlayerPawn 0)))
  (Variables|Default|SetVRPawn _asvrpawn)
  (CallFunction|FollowPlayer))

(event EventTick
  (params (DeltaSeconds :type Float%20%28single-precision%29))
  (if (< (Math|Vector|VectorLength (Pawn|Components|CharacterMovement|GetLastUpdateVelocity (Variables|Character|GetCharacterMovement))) 1e+01)
    _))

(fn ConstructionScript)