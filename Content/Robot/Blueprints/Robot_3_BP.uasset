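; Robot_3_BP is an AI-moved robot that wanders continuously and bumps Robot_2_BP robots on contact.
; Roam starts at BeginPlay, moves to a random reachable nearby point and calls itself on success.
; On failure it issues a wider-radius move and calls Roam again immediately, without waiting for that move.
; Hitting a Robot_2_BP prints "BUMP" and gives it a slight launch along this robot's forward vector.
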(event Custom|Roam
  (AI|AIMoveTo self (.RandomLocation (AI|Navigation|GetRandomReachablePointinRadius (Transformation|GetActorLocation) 4e+02 0 0)) 0 5.0 false
    (:OnSuccess
      _)
    (:OnFail
      (AI|AIMoveTo self (.RandomLocation (AI|Navigation|GetRandomReachablePointinRadius (Transformation|GetActorLocation) 6e+02 0 0)) 0 5.0 false
        (:then
          _))))
  (CallFunction|Roam))

(event EventBeginPlay
  (CallFunction|Roam))

(event Collision|EventHit
  (params (MyComp :type Primitive%20Component%20Object%20Reference) (Other :type Actor%20Object%20Reference) (OtherComp :type Primitive%20Component%20Object%20Reference) (bSelfMoved :type Boolean) (HitLocation :type Vector :default "0, 0, 0") (HitNormal :type Vector :default "0, 0, 0") (NormalImpulse :type Vector :default "0, 0, 0") (Hit :type Hit%20Result%20Structure%20%28by%20ref%29))
  (bind _asrobot_2_bp (Utilities|Casting|CastToRobot_2_BP Other))
  (Development|PrintString "BUMP")
  (Character|LaunchCharacter _asrobot_2_bp (* (Math|Vector|GetForwardVector (Transformation|GetActorRotation)) 2.0) false false))

(fn ConstructionScript)